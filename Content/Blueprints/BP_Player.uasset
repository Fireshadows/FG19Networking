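; Player Blueprint that shows its local network role and rocket count on a WBP_Role widget held by the WidgetRole component.
; On BeginPlay it converts the local role enum to text and writes it to the widget.
; OnNumRocketsChanged forwards each new count through SetNumRocketsinWidget to the widget, with no rocket logic in these graphs.
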(event `self.ReceiveBeginPlay`
  (bind _aswbp_role (cast `/Game/Blueprints/UI/WBP_Role` (`WidgetComponent.GetUserWidgetObject` (`self.Widget_Role`))))
  (`/Game/Blueprints/UI/WBP_Role.SetLocalText` _aswbp_role (`KismetTextLibrary.Conv_StringToText` (`|GetEnumeratorNameAsString` (`self.GetLocalRole`)))))

(event `Set Num Rockets in Widget`
  (params (`In Num Rockets` :type Integer))
  (bind _aswbp_role (cast `/Game/Blueprints/UI/WBP_Role` (`WidgetComponent.GetUserWidgetObject` (`self.Widget_Role`))))
  (`/Game/Blueprints/UI/WBP_Role.SetNumRockets` _aswbp_role `In Num Rockets`))

(event `self.BP_OnNumRocketsChanged`
  (params (NewNumRockets :type Integer))
  (`self.Set Num Rockets in Widget` NewNumRockets))

(fn `UserConstructionScript`)